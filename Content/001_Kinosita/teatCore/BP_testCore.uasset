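; BP_testCore is a test actor, driven as a pawn, that wanders endlessly around its starting location.
; BeginPlay stores that location, then AIMoveTo sends it to a random reachable navmesh point within MoveRadius of it.
; Success waits DelayNextMove and failure waits briefly, each printing a debug string and looping back to pick a new point.
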(event `self.ReceiveBeginPlay`
  (bind _output_get (set `self.StartLocation` (`self.K2_GetActorLocation`)))
  (bind _output_get_2 (set `self.Random Location` (`NavigationSystemV1.K2_GetRandomReachablePointInRadius` _output_get (`self.MoveRadius`) null null) :!label _label))
  (`|AIMoveTo` self _output_get_2 null
    (:`OnSuccess`
      (`KismetSystemLibrary.PrintString` "On Success")
      (`KismetSystemLibrary.Delay` (`self.DelayNextMove`))
      (goto _label))
    (:`OnFail`
      (`KismetSystemLibrary.PrintString` "On Fail")
      (`KismetSystemLibrary.Delay` 0.2)
      (goto _label))))

(fn `UserConstructionScript`)