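; BP_testEnemy is a test enemy that damages the player or the core through its AttackCollision overlap.
; The player takes heavier damage than the core, and either hit sets a longer StandbyTime than any other overlap.
; Every overlap then passes StandbyTime to the AI controller's blackboard and sets isBlock to true.
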(event `self.AttackCollision.OnComponentBeginOverlap`
  (params (OverlappedComponent :type "PrimitiveComponent Object Reference") (OtherActor :type "Actor Object Reference") (OtherComp :type "PrimitiveComponent Object Reference") (OtherBodyIndex :type Integer) (bFromSweep :type Boolean) (SweepResult :type "HitResult Structure (by ref)"))
  (bind _returnvalue (`GameplayStatics.GetPlayerCharacter` 0))
  (bind _bp_core (`self.BP_Core`))
  (if (== OtherActor _returnvalue)
    (`GameplayStatics.ApplyDamage` _returnvalue 10.0 null self) ; Player
    (set `self.StandbyTime` 5.0 :!label _label)
    (else
      (if (== OtherActor _bp_core)
        (`/Engine/EditorBlueprintResources/StandardMacros.IsValid` _bp_core
          (:`Is Valid`
            (`GameplayStatics.ApplyDamage` _bp_core 1.0 null self) ; core
            (goto _label))
          (:`Is Not Valid`
            _)))
      (set `self.StandbyTime` 1.0)))
  (`self.SetBlackboardValue`) ; ブラックボード変数の処理
)

(fn `SetBlackboardValue`
  (bind _returnvalue (`AIBlueprintHelperLibrary.GetBlackboard` (`AIBlueprintHelperLibrary.GetAIController` self)))
  (`BlackboardComponent.SetValueAsFloat` _returnvalue "StandbyTime" (`self.StandbyTime`))
  (`BlackboardComponent.SetValueAsBool` _returnvalue "isBlock" true))

(fn `UserConstructionScript`)