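; Boss character that always turns toward the player and runs parry-based melee combos whose length grows with its level.
; Combos draw random attack data assets without consecutive repeats; montage messages toggle a socket-attached hit sphere, and only a parry advances the chain.
; Parrying the finisher triggers a sequencer-actor rush, boss-only slow motion and knockback for a timed window.
; Damage counts only during break; window end checks HP for results or time-up game over.
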(event `self.ReceiveBeginPlay`
  (`BlackboardComponent.SetValueAsObject` (`AIBlueprintHelperLibrary.GetBlackboard` null) "playerActor" (`GameplayStatics.GetPlayerCharacter` 0))
  (`UserWidget.AddToViewport` (`self.WBP_HPBar`) 0)
  (bind _returnvalue (`GameplayStatics.GetActorOfClass` "/Game/003_Boushiyama/BP/seqActor.seqActor_C"))
  (set `self.BP_SeqActor` _returnvalue))

(event `self.ReceiveTick`
  (params (DeltaSeconds :type "Float (single-precision)"))
  (`self.K2_SetActorRotation` self (`KismetMathLibrary.RInterpTo` (`self.K2_GetActorRotation` self) (`KismetMathLibrary.MakeRotator` 0.0 0.0 (.yaw (`KismetMathLibrary.FindLookAtRotation` (`self.K2_GetActorLocation` self) (`self.K2_GetActorLocation` (`GameplayStatics.GetPlayerCharacter` 0))))) DeltaSeconds) false))

(event `/Game/000_Kidachi/BPI_Boss.Attack`
  (params (AIController :type "Actor Object Reference"))
  (set `self.AIController` AIController)
  (if (not (`self.bIsAttacking`))
    (`self.StartComboCycle` self)))

(event `/Game/000_Kidachi/BPI_Boss.Attack_Anim_FinishMsg`
  (`self.FinishCurrentAttack` self))

(event `/Game/000_Kidachi/BPI_Boss.Attack_Anim_HitStart`
  ;[1 1 1] 攻撃アニメーションが再生されたとき攻撃コリジョンを有効にする
  (`PrimitiveComponent.SetCollisionProfileName` (`self.AttackSphere`) "VisibleTrue" false))

(event `/Game/000_Kidachi/BPI_Boss.Attack_Anim_HitEnd`
  ;[1 1 1] 攻撃アニメーションが再生されたとき攻撃コリジョンを無効にする
  (`PrimitiveComponent.SetCollisionProfileName` (`self.AttackSphere`) "NoCollision" false))

(event `self.AttackSphere.OnComponentBeginOverlap`
  (params (OverlappedComponent :type "PrimitiveComponent Object Reference") (OtherActor :type "Actor Object Reference") (OtherComp :type "PrimitiveComponent Object Reference") (OtherBodyIndex :type Integer) (bFromSweep :type Boolean) (SweepResult :type "HitResult Structure (by ref)"))
  (bind _returnvalue (`GameplayStatics.GetPlayerCharacter` 0))
  (if (== OtherActor _returnvalue)
    (`GameplayStatics.ApplyDamage` _returnvalue (`/Game/002_Onishi/DataAsset/PDA_BossAttackBase.Damage` (`self.CurrentAttackData`)) null self)
    ;[1 1 1] パリィ失敗
    (set `self.bCurrentAttackHitPlayer` false)
    (set `self.bComboAllParried` false)
    (if (`self.bTimeUp`)
      (set `self.bLastChanceMode` false))))

(event `/Game/000_Kidachi/BPI_Boss.ParrySuccess`
  ;[1 1 1] パリィが成功したらコリジョンを無効化する
  (`PrimitiveComponent.SetCollisionProfileName` (`self.AttackSphere`) "NoCollision" true)
  (set `self.bCurrentAttackWasParried` true)
  (set `self.bAttackHitActive` false)
  ;[1 1 1] パリィが最終段かどうか判定
  (if (== (`KismetArrayLibrary.Array_LastIndex` (`self.GeneratedCombo`)) (`self.CurrentComboIndex`))
    (set `self.bPendingFinalParryReaction` true)
    (`/Game/003_Boushiyama/BP/seqActor.RushStart` (`self.BP_SeqActor`) (0.0 0.0 0.0))
    ;[1 1 1] スローモーション開始
    (`self.StartBossSlowMotion`)
    (set `self.Direction` (- (`self.K2_GetActorLocation`) (`self.K2_GetActorLocation` (`GameplayStatics.GetPlayerCharacter` 0))))
    (`/Game/003_Boushiyama/BP/seqActor.RushStart` (`self.BP_SeqActor`) (`self.Direction`))
    ;[1 1 1] 怯みモーションを再生
    (`self.StopAnimMontage` (`/Game/002_Onishi/DataAsset/PDA_BossAttackBase.AttackMontage` (`self.CurrentAttackData`)))
    (`self.PlayAnimMontage` "/Game/boss/bossAnimation/AnimationMontage/AN_Boss_Damage.AN_Boss_Damage")
    (`KismetSystemLibrary.K2_SetTimerDelegate` (delegate `TestSlowMotion`) 10.0)
    ;[1 1 1] プレイヤーの位置に合わせてノックバックする
    (`self.LaunchCharacter` (* (`KismetMathLibrary.Normal` (- (`self.K2_GetActorLocation`) (`self.K2_GetActorLocation` (`GameplayStatics.GetPlayerCharacter` 0))) 1.0) (`self.ParryKnockbackPower`)) true)))

(event `TestSlowMotion`
  (`self.EndBossBreak` self))

(event `self.LastDeath`
  (set `self.bTimeUp` true)
  (if (`self.bIsBreak`)
    (set `self.bTimeUpRequested ` true)
    (else
      (set `self.bLastChanceMode` true))))

(event `self.ReceiveAnyDamage`
  (params (Damage :type "Float (single-precision)") (DamageType :type "DamageType Object Reference") (InstigatedBy :type "Controller Object Reference") (DamageCauser :type "Actor Object Reference"))
  ;[1 1 1] ダメージ処理
  (if (`self.bIsBreak`)
    (set `self.HP` (- (`self.HP`) Damage))))

(fn `CheckRushResultAfterBreak`
  (if (< (`self.HP`) 0.0)
    (`GameplayStatics.OpenLevel` "L_Result")
    (elif (`self.bTimeUpRequested `)
      (bind _returnvalue (`|CreateWidget` "/Game/005_Kidani/BP/WBP_Over.WBP_Over_C"))
      (`UserWidget.AddToViewport` _returnvalue 0))))

(fn `EndBossBreak`
  (`self.EndBossSlowMotion` self)
  (`self.CheckRushResultAfterBreak` self)
  (`self.RequestTimeUpGameOver` self))

(fn `EndBossSlowMotion`
  (set `self.bBossSlowMotion` false)
  (set `self.CustomTimeDilation` 1.0))

(fn `FinishCurrentAttack`
  (set `self.bCanParry` false)
  (set `self.bAttackHitActive` false)
  (if (`self.bCurrentAttackHitPlayer`)
    (`self.ParryFaild`)
    (if (`self.bLastChanceMode`)
      (bind _returnvalue (`|CreateWidget` "/Game/005_Kidani/BP/WBP_Over.WBP_Over_C"))
      (`UserWidget.AddToViewport` _returnvalue 0))
    (elif (`self.bCurrentAttackWasParried`)
      (if (== (`self.CurrentComboIndex`) (- (`KismetArrayLibrary.Array_Length` (`self.GeneratedCombo`)) 1))
        (if (>= (`self.CurrentLevel`) (`self.MaxComboLevel`))
          (set `self.CurrentLevel` 1)
          (else
            (`/Engine/EditorBlueprintResources/StandardMacros.IncrementInt` (`self.CurrentLevel`)
              (:`  `
                _))))
        (set `self.CurrentComboIndex` 0)
        (set `self.bIsAttacking` false)
        (message `/Game/000_Kidachi/BPI_BossAI.FinishAttack` (`self.AIController`))
        (else
          (`/Engine/EditorBlueprintResources/StandardMacros.IncrementInt` (`self.CurrentComboIndex`)
            (:`  `
              (`self.SelectNextAttackData`)
              (`self.StartCurrentAttack`)))))
      (else
        (`self.ParryFaild`)
        (if (`self.bLastChanceMode`)
          (bind _returnvalue_2 (`|CreateWidget` "/Game/005_Kidani/BP/WBP_Over.WBP_Over_C"))
          (`UserWidget.AddToViewport` _returnvalue_2 0))))))

(fn `GenerateCombo`
  (bind _output (`|GetArrayItem` (`self.CandidateList`) (`self.RandomIndex`)))
  (`KismetArrayLibrary.Array_Clear` (`self.GeneratedCombo`))
  (set `self.CurrentComboIndex` 0)
  (set `self.CurrentComboLength` (`KismetMathLibrary.Clamp` (`self.CurrentLevel`) 1 3))
  (for _ (range (`self.CurrentComboLength`))
    (`KismetArrayLibrary.Array_Clear` (`self.CandidateList`))
    (for _array_element (`self.AttackDataList`)
      (`/Engine/EditorBlueprintResources/StandardMacros.IsValid` _array_element
        (:`Is Valid`
          (`/Engine/EditorBlueprintResources/StandardMacros.IsValid` (`self.LocalLastAttackData`)
            (:`Is Valid`
              ;[1 1 1] 同じ攻撃データを繰り返さないようにする
              (if (not (`|EnumEquality` (`/Game/002_Onishi/DataAsset/PDA_BossAttackBase.AttackType` _array_element) (`/Game/002_Onishi/DataAsset/PDA_BossAttackBase.AttackType` (`self.LocalLastAttackData`))))
                (`KismetArrayLibrary.Array_Add` (`self.CandidateList`) _array_element)))
            (:`Is Not Valid`
              (`KismetArrayLibrary.Array_Add` (`self.CandidateList`) _array_element))))))
    (if (> (`KismetArrayLibrary.Array_Length` (`self.CandidateList`)) 0)
      (set `self.RandomIndex` (`KismetMathLibrary.RandomIntegerInRange` 0 (- (`KismetArrayLibrary.Array_Length` (`self.CandidateList`)) 1)))
      (`KismetArrayLibrary.Array_Add` (`self.GeneratedCombo`) _output)
      (set `self.LocalLastAttackData` _output))))

(fn `GetRushPos`
  (returns (RushPos :type "Vector Structure"))
  (return (`SceneComponent.K2_GetComponentLocation` (`self.RushTargetPoint`))))

(fn `ParryFaild`
  (set `self.bComboAllParried` false)
  (set `self.CurrentComboIndex` 0)
  (set `self.bIsAttacking` false)
  (message `/Game/000_Kidachi/BPI_BossAI.FinishAttack` (`self.AIController`)))

(fn `RequestTimeUpGameOver`
  (if (`self.bIsBreak`)
    (set `self.bTimeUpRequested ` true)
    (else
      (`KismetSystemLibrary.PrintString` "GameOver"))))

(fn `SelectNextAttackData`
  (if (> (`KismetArrayLibrary.Array_Length` (`self.GeneratedCombo`)) 0)
    (if (and (>= (`self.CurrentComboIndex`) 0) (< (`self.CurrentComboIndex`) (`KismetArrayLibrary.Array_Length` (`self.GeneratedCombo`))))
      (bind _output_get (set `self.CurrentAttackData` (`|GetArrayItem` (`self.GeneratedCombo`) (`self.CurrentComboIndex`))))
      (set `self.CurrentAttackType` (`/Game/002_Onishi/DataAsset/PDA_BossAttackBase.AttackType` _output_get))
      (set `self.bCurrentAttackHitPlayer` false)
      (set `self.bCurrentAttackWasParried` false)
      (set `self.bCanParry` false)
      (set `self.bAttackHitActive` false)
      (set `self.bIsCurrentAttackFinisher` (== (`self.CurrentComboIndex`) (- (`self.CurrentComboLength`) 1)))
      (else
        (set `self.CurrentAttackData` null)
        (set `self.bIsCurrentAttackFinisher` false)
        (return)))
    (else
      (set `self.CurrentAttackData` null)
      (set `self.bIsCurrentAttackFinisher` false)
      (return))))

(fn `StartBossSlowMotion`
  (set `self.bBossSlowMotion` true)
  (set `self.CustomTimeDilation` (`self.BossSlowMotionRate`)))

(fn `StartComboCycle`
  (set `self.bComboAllParried` true)
  (`self.GenerateCombo` self)
  (`self.SelectNextAttackData` self)
  (`self.StartCurrentAttack` self))

(fn `StartCurrentAttack`
  (locals (MontageToPlay :type "AnimMontage Object Reference"))
  (`/Engine/EditorBlueprintResources/StandardMacros.IsValid` (`self.CurrentAttackData`)
    (:`Is Valid`
      (set `self.bIsAttacking` true)
      (set `self.bCanParry` false)
      (set `self.bAttackHitActive` false)
      (set `self.bCurrentAttackHitPlayer` false)
      (set `self.bCurrentAttackWasParried` false)
      (bind _output_get (set `local.MontageToPlay` (`/Game/002_Onishi/DataAsset/PDA_BossAttackBase.AttackMontage` (`self.CurrentAttackData`))))
      (if (`KismetSystemLibrary.IsValid` _output_get)
        (`SceneComponent.K2_AttachToComponent` (`self.AttackSphere`) (`self.Mesh`) (`/Game/002_Onishi/DataAsset/PDA_BossAttackBase.SoketName` (`self.CurrentAttackData`)) "KeepRelative" "KeepRelative" "KeepRelative" true)
        (bind _returnvalue (`self.PlayAnimMontage` (`local.MontageToPlay`)))
        (if (not (> _returnvalue 0.0))
          (set `self.bIsAttacking` false)
          (`KismetSystemLibrary.PrintString` "\"Montage Play Failed\""))
        (else
          (set `self.bIsAttacking` false)
          (`KismetSystemLibrary.PrintString` "\"StartCurrentAttack: MontageToPlay is Invalid\""))))
    (:`Is Not Valid`
      (set `self.bIsAttacking` false))))

(fn `UserConstructionScript`)