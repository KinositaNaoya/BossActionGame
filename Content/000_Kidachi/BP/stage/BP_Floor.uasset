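; BP_Floor is a floor actor that keeps a square grid of tiles around the player, giving the effect of an endless floor.
; BeginPlay creates the grid as InstancedStaticMesh instances, storing each one's tile coordinate in TilePos.
; When the player's tile changes, Tick shifts every coordinate by that delta and moves the existing instances instead of spawning new ones.
; CulcWorldPos offsets odd rows by half a tile, forming a staggered layout.
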(event `self.ReceiveBeginPlay`
  (bind _maxtilenum (`self.maxTileNum`))
  (bind _returnvalue (/ (`self.maxTileNum`) 2))
  (set `self.OldPlayerPos` (make `IntPoint` 0))
  (for _index (range (* _maxtilenum _maxtilenum))
    (bind _returnvalue_2 (- (/ _index (`self.maxTileNum`)) _returnvalue))
    (bind _returnvalue_3 (- (mod _index (`self.maxTileNum`)) _returnvalue))
    (bind _position (`self.CulcWorldPos` (make `IntPoint` _returnvalue_2 _returnvalue_3)))
    (bind _returnvalue_4 (`InstancedStaticMeshComponent.AddInstance` (`self.InstancedStaticMesh`) (`KismetMathLibrary.MakeTransform` (`KismetMathLibrary.MakeVector` (`KismetMathLibrary.BreakVector2D` _position) (`.Y` (`KismetMathLibrary.BreakVector2D` _position))) (struct) (30.0 30.0 0.5)) true))
    (`BlueprintMapLibrary.Map_Add` (`self.TilePos`) _returnvalue_4 (make `IntPoint` _returnvalue_2 _returnvalue_3))))

(event `self.ReceiveTick`
  (params (DeltaSeconds :type "Float (single-precision)"))
  (bind _maxtilenum (`self.maxTileNum`))
  (bind (_returnvalue_x _returnvalue_y) (`KismetMathLibrary.BreakVector` (`self.K2_GetActorLocation` (`GameplayStatics.GetPlayerCharacter` 0))))
  (bind (_returnvalue_x_2 _returnvalue_y_2) (break `IntPoint` (- (`self.CurrentPlayerPos`) (`self.OldPlayerPos`))))
  (bind _tilepos (`self.GetTilePos` (`KismetMathLibrary.MakeVector2D` _returnvalue_x _returnvalue_y)))
  (set `self.CurrentPlayerPos` _tilepos)
  (if (not (`KismetMathLibrary.Equal_IntPointIntPoint` _tilepos (`self.OldPlayerPos`)))
    (`|ExecutionSequence`
      (:`then_0`
        ;[1 1 1] 移動
        (for _index (range (* _maxtilenum _maxtilenum))
          (bind _returnvalue (+ (`BlueprintMapLibrary.Map_Find` (`self.TilePos`) _index) (`KismetMathLibrary.MakeVector2D` (`KismetMathLibrary.Conv_IntToDouble` _returnvalue_x_2) (`KismetMathLibrary.Conv_IntToDouble` _returnvalue_y_2))))
          (bind _position (`self.CulcWorldPos` _returnvalue))
          (`InstancedStaticMeshComponent.UpdateInstanceTransform` (`self.InstancedStaticMesh`) _index (`KismetMathLibrary.MakeTransform` (`KismetMathLibrary.MakeVector` (`KismetMathLibrary.BreakVector2D` _position) (`.Y` (`KismetMathLibrary.BreakVector2D` _position))) (struct) (30.0 30.0 0.5)) true true true)
          (`BlueprintMapLibrary.Map_Add` (`self.TilePos`) _index _returnvalue)))
      (:`then_1`
        (set `self.OldPlayerPos` (`self.CurrentPlayerPos`))))))

(fn `CulcWorldPos`
  (params (TilePos :type "IntPoint Structure"))
  (returns (Position :type "Vector2D Structure"))
  (bind (_tilesize_x _tilesize_y) (`KismetMathLibrary.BreakVector2D` (`self.TileSize`)))
  (return (`KismetMathLibrary.MakeVector2D` (+ (* TilePos_X _tilesize_x) (* (`KismetMathLibrary.Abs_Int` (mod TilePos_Y 2)) (/ _tilesize_x 2.0))) (* TilePos_Y _tilesize_y))))

(fn `GetTilePos`
  (params (Position :type "Vector2D Structure"))
  (returns (TilePos :type "IntPoint Structure"))
  (return (/ Position (`self.TileSize`))))

(fn `UserConstructionScript`)