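; BP_UIActor is an actor that manages game UI: title screen, 3D HP display, jump gauge and game-over screen.
; BeginPlay shows the title in UI-only input and, if a BP_3DUI exists, creates a hidden jump gauge and switches to the title camera.
; Events forward HP to BP_3DUI, set a rush flag, and start, judge and end the gauge animation.
; GameOver clears all widgets, shows WBP_Over and pauses.
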(event `self.ReceiveBeginPlay`
  (bind _returnvalue (`GameplayStatics.GetPlayerController` 0))
  (bind _returnvalue_2 (`|CreateWidget` "/Game/005_Kidani/BP/WBP_Title.WBP_Title_C"))
  (`UserWidget.AddToViewport` _returnvalue_2 0)
  (`WidgetBlueprintLibrary.SetInputMode_UIOnlyEx` _returnvalue null)
  (set `PlayerController.bShowMouseCursor` true _returnvalue)
  (bind _returnvalue_3 (`GameplayStatics.GetActorOfClass` "/Game/005_Kidani/BP/BP_3DUI.BP_3DUI_C"))
  (`/Engine/EditorBlueprintResources/StandardMacros.IsValid` _returnvalue_3
    (:`Is Valid`
      (set `self.as BP_3DUI` _returnvalue_3)
      (bind _returnvalue_4 (`|CreateWidget` "/Game/005_Kidani/BP/WBP_JumpGauge.WBP_JumpGauge_C"))
      (bind _output_get (set `self.JumpGauge_Ref` _returnvalue_4))
      (`UserWidget.AddToViewport` _output_get 0)
      (`Widget.SetVisibility` (`self.JumpGauge_Ref`) "Hidden")
      (bind _returnvalue_5 (`GameplayStatics.GetActorOfClass` "/Game/005_Kidani/BP/BP_TitleCamera.BP_TitleCamera_C"))
      (`PlayerController.SetViewTargetWithBlend` (`GameplayStatics.GetPlayerController` 0) _returnvalue_5 0.0 "VTBlend_Linear" 0.0 false))))

(event `InitalizeHp`
  (params (MaxHp :type "Float (double-precision)"))
  (`/Game/005_Kidani/BP/BP_3DUI.B_Initialize_3DHP` (`self.as BP_3DUI`) MaxHp))

(event `UpdateHp`
  (params (Hp :type "Float (double-precision)"))
  (`/Game/005_Kidani/BP/BP_3DUI.B_Update_3DHP` (`self.as BP_3DUI`) Hp))

(event `RushStrat`
  (set `self.isRush` true))

(event `GameOver`
  (bind _returnvalue (`GameplayStatics.GetPlayerController` 0))
  ;[1 0 0.08766] ゲームオーバーイベント
  (`WidgetLayoutLibrary.RemoveAllWidgets`)
  (bind _returnvalue_2 (`|CreateWidget` "/Game/005_Kidani/BP/WBP_Over.WBP_Over_C"))
  (`UserWidget.AddToViewport` _returnvalue_2 0)
  (`WidgetBlueprintLibrary.SetInputMode_UIOnlyEx` _returnvalue null)
  (set `PlayerController.bShowMouseCursor` true _returnvalue)
  (`GameplayStatics.SetGamePaused` true))

(event `StartJumpGauge`
  (bind _jumpgauge_ref (`self.JumpGauge_Ref`))
  ;[0.2903 1 0.1536] ジャンプゲージアニメーション
  (`/Game/005_Kidani/BP/WBP_JumpGauge.StartAnim` _jumpgauge_ref)
  (`UserWidget.BindToAnimationFinished` _jumpgauge_ref (`/Game/005_Kidani/BP/WBP_JumpGauge.MoveGreen` _jumpgauge_ref) (delegate `Finished`)))

(event `Finished`
  ;[0.2903 1 0.1536] ジャンプゲージアニメーション
  (`/Game/005_Kidani/BP/WBP_JumpGauge.EndAnim` (`self.JumpGauge_Ref`)))

(event `PressGauge`
  ;[0.2903 1 0.1536] ジャンプゲージアニメーション
  (`/Game/005_Kidani/BP/WBP_JumpGauge.AnimJudge` (`self.JumpGauge_Ref`)))

(fn `UserConstructionScript`)