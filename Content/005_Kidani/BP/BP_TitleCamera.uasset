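; Title-screen camera actor that continuously orbits a referenced center actor.
; Each Tick it advances an angle by RotationSpeed and places itself on a horizontal circle of OrbitRadius at the center actor's height, using sine and cosine.
; It then turns to face the center actor with FindLookAtRotation, following that actor if it moves.
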(event `self.ReceiveTick`
  (params (DeltaSeconds :type "Float (single-precision)"))
  (bind (_returnvalue_x _returnvalue_y _returnvalue_z) (`KismetMathLibrary.BreakVector` (`self.K2_GetActorLocation` (`self.OrbitCenterActor`))))
  (bind _returnvalue (`KismetMathLibrary.DegreesToRadians` (`self.CurrentAngle`)))
  (set `self.CurrentAngle` (+ (`self.CurrentAngle`) (* (`self.RotationSpeed`) DeltaSeconds)))
  (`self.K2_SetActorLocation` (`KismetMathLibrary.MakeVector` (+ (* (`KismetMathLibrary.Cos` _returnvalue) (`self.OrbitRadius`)) _returnvalue_x) (+ (* (`KismetMathLibrary.Sin` _returnvalue) (`self.OrbitRadius`)) _returnvalue_y) _returnvalue_z))
  (`self.K2_SetActorRotation` (`KismetMathLibrary.FindLookAtRotation` (`self.K2_GetActorLocation`) (`self.K2_GetActorLocation` (`self.OrbitCenterActor`)))))

(fn `UserConstructionScript`)