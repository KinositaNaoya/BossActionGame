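; BP_OrbitCenter is an actor that marks the center of an orbit for the title camera.
; Its Sphere component is sized to OrbitRadius in both the construction script and BeginPlay, so the sphere matches the orbit.
; On BeginPlay it spawns a BP_TitleCamera at its own location and passes it itself as orbit center, along with the radius and rotation speed.
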(event `self.ReceiveBeginPlay`
  (`SphereComponent.SetSphereRadius` (`self.Sphere`) (`self.OrbitRadius`) true)
  (bind _returnvalue (`|SpawnActorFromClass` "/Game/005_Kidani/BP/BP_TitleCamera.BP_TitleCamera_C" (`KismetMathLibrary.Conv_VectorToTransform` (`self.K2_GetActorLocation`)) "Undefined" "MultiplyWithRoot" null null))
  (set `self.Camera_Ref` _returnvalue)
  (set `/Game/005_Kidani/BP/BP_TitleCamera.OrbitCenterActor` self (`self.Camera_Ref`))
  (set `/Game/005_Kidani/BP/BP_TitleCamera.OrbitRadius` (`self.OrbitRadius`) (`self.Camera_Ref`))
  (set `/Game/005_Kidani/BP/BP_TitleCamera.RotationSpeed` (`self.RotationSpeed`) (`self.Camera_Ref`)))

(fn `UserConstructionScript`
  (`SphereComponent.SetSphereRadius` (`self.Sphere`) (`self.OrbitRadius`) true))