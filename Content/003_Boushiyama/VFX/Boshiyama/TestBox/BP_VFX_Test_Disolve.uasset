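; Test Blueprint for a dissolve VFX on a cube, triggered by overlapping a box.
; Box overlap plays a timeline that drives the cube's EmissiveTime material parameter, and ending the overlap reverses the timeline from its end.
; Each timeline update also switches the cube's collision object type between two custom channels, depending on whether the track value has reached one.
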(event `self.Box.OnComponentBeginOverlap`
  (params (OverlappedComponent :type "PrimitiveComponent Object Reference") (OtherActor :type "Actor Object Reference") (OtherComp :type "PrimitiveComponent Object Reference") (OtherBodyIndex :type Integer) (bFromSweep :type Boolean) (SweepResult :type "HitResult Structure (by ref)"))
  (bind (_direction `_新規track_0`) (`Timeline|タイムライン` :!label _label)
    (:`Update`
      (`MeshComponent.SetScalarParameterValueOnMaterials` (`self.Cube`) "EmissiveTime" `_新規track_0`)
      (if (>= `_新規track_0` 1.0)
        (`PrimitiveComponent.SetCollisionObjectType` (`self.Cube`) "ECC_GameTraceChannel2")
        (else
          (`PrimitiveComponent.SetCollisionObjectType` (`self.Cube`) "ECC_GameTraceChannel3"))))))

(event `self.Box.OnComponentEndOverlap`
  (params (OverlappedComponent :type "PrimitiveComponent Object Reference") (OtherActor :type "Actor Object Reference") (OtherComp :type "PrimitiveComponent Object Reference") (OtherBodyIndex :type Integer))
  (goto _label :!via `ReverseFromEnd`))

(fn `UserConstructionScript`)