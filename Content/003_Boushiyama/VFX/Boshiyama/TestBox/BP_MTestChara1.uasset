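; BP_MTestChara1 is a VFX test character that plays an animation montage on its mesh when something begins overlapping its box.
; An unconnected chain would ragdoll the mesh with physics, then run a timeline driving a dissolve-style "Animetion" material parameter and a Niagara "User_Animation" float, destroying the actor when finished.
; BeginPlay, end overlap and the construction script are empty.
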(event `self.ReceiveBeginPlay`)

(event `self.Box.OnComponentBeginOverlap`
  (params (OverlappedComponent :type "PrimitiveComponent Object Reference") (OtherActor :type "Actor Object Reference") (OtherComp :type "PrimitiveComponent Object Reference") (OtherBodyIndex :type Integer) (bFromSweep :type Boolean) (SweepResult :type "HitResult Structure (by ref)"))
  (`|PlayMontage` (`self.Mesh`) (`self.Montage to Play`)))

(event `self.Box.OnComponentEndOverlap`
  (params (OverlappedComponent :type "PrimitiveComponent Object Reference") (OtherActor :type "Actor Object Reference") (OtherComp :type "PrimitiveComponent Object Reference") (OtherBodyIndex :type Integer)))

(fn `UserConstructionScript`)